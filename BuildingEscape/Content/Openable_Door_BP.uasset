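; Openable door actor that swings open and shut in response to OnOpen and OnClose events from its OpenDoor member.
; It stores its starting rotation at BeginPlay, then the DoorSwing timeline's OpenAngle track offsets the actor's yaw from that rotation through DeltaRotator.
; Opening plays the timeline and closing reverses it, with a Sound Cue event track playing the door lock sound at the actor's location.
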(event OnOpen(OpenDoor)
  (bind _open_angle (Timeline|Door%20Swing Play)
    (:Update
      (Transformation|SetActorRotation (Math|Rotator|Delta(Rotator) (Variables|Default|GetInitial%20Rotation) (Math|Rotator|MakeRotator 0.0 0.0 _open_angle))))
    (:SoundCue
      (Audio|PlaySoundatLocation "/Game/Audio/door-lock.door-lock" (Transformation|GetActorLocation)))))

(event OnClose(OpenDoor)
  (bind _open_angle (Timeline|Door%20Swing Reverse)
    (:Update
      (Transformation|SetActorRotation (Math|Rotator|Delta(Rotator) (Variables|Default|GetInitial%20Rotation) (Math|Rotator|MakeRotator 0.0 0.0 _open_angle))))
    (:SoundCue
      (Audio|PlaySoundatLocation "/Game/Audio/door-lock.door-lock" (Transformation|GetActorLocation)))))

(event EventBeginPlay
  (Variables|Default|SetInitial%20Rotation (Transformation|GetActorRotation)))

(fn ConstructionScript)